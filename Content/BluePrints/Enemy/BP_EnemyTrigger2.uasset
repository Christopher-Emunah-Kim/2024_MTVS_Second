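; BP_EnemyTrigger2 is a one-shot box trigger that spawns a wave of enemies when the player (BP_JPlayer) overlaps it.
; It finds factory actors tagged EnemyFactory by class, then calls spawn on one clicker factory and two normal factories chosen by hard-coded array index.
; The trigger destroys itself afterwards, and the factory selection depends on the order GetAllActorsOfClassWithTag returns.
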(event OnComponentBeginOverlap(Box)
  (params (OverlappedComponent :type Primitive%20Component%20Object%20Reference) (OtherActor :type Actor%20Object%20Reference) (OtherComp :type Primitive%20Component%20Object%20Reference) (OtherBodyIndex :type Integer) (bFromSweep :type Boolean) (SweepResult :type Hit%20Result%20Structure%20%28by%20ref%29))
  (Utilities|Casting|CastToBP_JPlayer OtherActor)
  (if true
    (Utilities|FlowControl|Sequence
      (:then_0
        (bind _outactors (Actor|GetAllActorsOfClasswithTag "/Game/BluePrints/Enemy/BP_ClickerEnemyFactory.BP_ClickerEnemyFactory_C" "EnemyFactory"))
        (Default|SpawnClickerEnemy (Utilities|Array|Get(acopy) _outactors)))
      (:then_1
        (bind _outactors_2 (Actor|GetAllActorsOfClasswithTag "/Game/BluePrints/Enemy/BP_NormalEnemyFactory.BP_NormalEnemyFactory_C" "EnemyFactory"))
        (Default|SpawnNormalEnemy (Utilities|Array|Get(acopy) _outactors_2 2)))
      (:then_2
        (bind _outactors_3 (Actor|GetAllActorsOfClasswithTag "/Game/BluePrints/Enemy/BP_NormalEnemyFactory.BP_NormalEnemyFactory_C" "EnemyFactory"))
        (Default|SpawnNormalEnemy (Utilities|Array|Get(acopy) _outactors_3 3)))
      (:then_3
        (Actor|DestroyActor)))))

(event EventBeginPlay)

(event Collision|EventActorBeginOverlap
  (params (OtherActor :type Actor%20Object%20Reference)))

(event EventTick
  (params (DeltaSeconds :type Float%20%28single-precision%29)))

(fn ConstructionScript)