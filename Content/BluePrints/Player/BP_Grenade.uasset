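; BP_Grenade is a thrown firebomb that spawns a BP_BurningField at the impact point when its sphere overlaps something, then destroys itself.
; Throw runs once, either when called or automatically after a BeginPlay delay, detaching the actor and launching it through ProjectileMovement.
; Sphere collision starts disabled and turns on shortly after launch, when a limited lifespan is also set.
; The Cube component rotates toward a random rotation during flight.
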(event OnComponentBeginOverlap(Sphere)
  (params (OverlappedComponent :type Primitive%20Component%20Object%20Reference) (OtherActor :type Actor%20Object%20Reference) (OtherComp :type Primitive%20Component%20Object%20Reference) (OtherBodyIndex :type Integer) (bFromSweep :type Boolean) (SweepResult :type Hit%20Result%20Structure%20%28by%20ref%29))
  ;[1 1 1] 닿으면 불 스폰
  (Game|SpawnActorfromClass "/Game/BluePrints/Player/BP_BurningField.BP_BurningField_C" (Math|Conversions|ToTransform(Vector) (.impactpoint SweepResult)) "Undefined" "MultiplyWithRoot" 0 0)
  (Actor|DestroyActor))

(event Custom|Throw
  (params (Velocity :type Vector))
  (bind _projectilemovement (Variables|Default|GetProjectileMovement))
  (Utilities|FlowControl|DoOnce false
    (:Completed
      (Utilities|FlowControl|Sequence
        (:then_0
          ;[1 1 1] 액터로부터 떼고 날리기
          (Transformation|DetachFromActor "KeepWorld" "KeepWorld" "KeepWorld")
          ;[1 1 1] 화염병 날리고 0.2초 뒤에 콜리전 활성화
          (Variables|/Script/Engine.MovementComponent|SetVelocity _projectilemovement Velocity)
          (Components|Activation|Activate _projectilemovement false)
          (Utilities|FlowControl|Delay 0.2)
          (Collision|SetCollisionEnabled (Variables|Default|GetSphere) "QueryAndPhysics")
          (Actor|SetLifeSpan 3.0))
        (:then_1
          (Components|MoveComponentTo (Variables|Default|GetCube) "0, 0, 0" (Math|Random|RandomRotator false) false false 15.0 false))))))

(event EventBeginPlay
  (Utilities|FlowControl|Delay 2.0)
  (CallFunction|Throw (* (Transformation|GetActorForwardVector) 1.5e+03)))

(fn ConstructionScript
  (Collision|SetCollisionEnabled (Variables|Default|GetSphere) "NoCollision"))