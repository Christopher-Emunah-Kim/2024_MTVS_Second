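; BP_AttackCollision is an animation notify state that opens the player's attack hit window during a montage or animation.
; On begin it sets BP_JPlayer's left and right attack spheres to QueryAndPhysics collision, and on end it disables both.
; It finds the player with GetActorOfClass rather than the mesh's owner, so it always affects the first BP_JPlayer found.
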(fn ReceivedNotifyEnd
  (params (MeshComp :type Skeletal%20Mesh%20Component%20Object%20Reference) (Animation :type Anim%20Sequence%20Base%20Object%20Reference) (EventReference :type Anim%20Notify%20Event%20Reference%20Structure%20%28by%20ref%29))
  (bind _returnvalue (Actor|GetActorOfClass MeshComp "/Game/BluePrints/Player/BP_JPlayer.BP_JPlayer_C"))
  (Collision|SetCollisionEnabled (Variables|/Script/LastOfNN.JPlayer|GetRightAttackSphere _returnvalue) "NoCollision")
  (Collision|SetCollisionEnabled (Variables|/Script/LastOfNN.JPlayer|GetLeftAttackSphere _returnvalue) "NoCollision")
  (return false))

(fn ReceivedNotifyBegin
  (params (MeshComp :type Skeletal%20Mesh%20Component%20Object%20Reference) (Animation :type Anim%20Sequence%20Base%20Object%20Reference) (TotalDuration :type Float%20%28single-precision%29) (EventReference :type Anim%20Notify%20Event%20Reference%20Structure%20%28by%20ref%29))
  (bind _returnvalue (Actor|GetActorOfClass MeshComp "/Game/BluePrints/Player/BP_JPlayer.BP_JPlayer_C"))
  (Collision|SetCollisionEnabled (Variables|/Script/LastOfNN.JPlayer|GetRightAttackSphere _returnvalue) "QueryAndPhysics")
  (Collision|SetCollisionEnabled (Variables|/Script/LastOfNN.JPlayer|GetLeftAttackSphere _returnvalue) "QueryAndPhysics")
  (return false))