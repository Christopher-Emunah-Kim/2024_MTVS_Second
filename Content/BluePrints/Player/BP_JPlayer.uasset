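; Player character Blueprint that handles aiming and throwing Molotov cocktails (BP_Grenade) while a throw weapon is equipped.
; Left mouse press plays a standing or crouched throw montage and spawns the projectile attached to the right hand.
; While held, a predicted trajectory is rebuilt every frame as spline meshes with a debug landing sphere.
; Release jumps to the montage's Throw section, then launches BPGrenade after a short delay and decrements ammo.
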(event Custom|ShowProjectTilePath
  (bind _projectile_path (Variables|Default|GetProjectile%20Path))
  (|ClearPath
    (:Completed
      (if (Variables|Default|GetThrowing)
        (bind (_outhit _outpathpositions _outlasttracedestination) (Class|GameplayStatics|BlueprintPredictProjectilePathbyTraceChannel (Transformation|GetWorldLocation (Variables|Default|GetProjectile%20Start)) (Utilities|ThrowVelicity) true 1.0 "ECC_Camera" false (Utilities|Array|MakeArray self) "None" 0.0 1e+01))
        (for (_array_element _array_index) _outpathpositions
          (Spline|AddSplinePointatIndex (Variables|Default|GetProjectile%20Path) _array_element _array_index "Local" true))
        (for _index (range 0 (- (Spline|GetNumberOfSplinePoints (Variables|Default|GetProjectile%20Path)) 2))
          ;[1 1 1] 이게 문제구나
          (bind _returnvalue (AddComponent|AddSplineMeshComponent true))
          (SplineMesh|SetStartandEnd _returnvalue (Spline|GetLocationatSplinePoint _projectile_path _index "Local") (Spline|GetTangentatSplinePoint _projectile_path _index "Local") (Spline|GetLocationatSplinePoint _projectile_path (+ _index 1) "Local") (Spline|GetTangentatSplinePoint _projectile_path (+ _index 1) "Local") true :!class /Script/Engine.SplineMeshComponent)
          (Utilities|Array|Add (Variables|Default|GetSplineMesh%20Components) _returnvalue))
        ;[1 1 1] 경로 예상 초기화 후 재생성(화면 돌렸을때)
        (Utilities|FlowControl|Delay (Utilities|Time|GetWorldDeltaSeconds))
        (CallFunction|ShowProjectTilePath)
        (Rendering|Debug|DrawDebugSphere (+ _outlasttracedestination "0.000000,0.000000,50.000000") 4e+01 12 "(R=0.000000,G=120.000000,B=0.000000,A=1.000000)" 0.1 2.0)))))

(event EventTick
  (params (DeltaSeconds :type Float%20%28single-precision%29)))

(event Input|MouseEvents|LeftMouseButton
  (params (Key :type Key%20Structure :default "None"))
  (bind _bp_grenade (Variables|Default|GetBP%20Grenade))
  (bind _characterequipstate (Variables|Default|GetCharacterEquipState))
  (bind _mesh (Variables|Character|GetMesh))
  (bind _returnvalue (Components|SkeletalMesh|GetAnimInstance _mesh))
  (bind _returnvalue_2 (Utilities|Enum|Equal(Enum) _characterequipstate "ECES_ThrowWeaponEquipped"))
  (:Pressed
    (if (!= 0 (Variables|Default|GetMolotovcocktailNum))
      (if _returnvalue_2
        (Variables|Default|SetThrowing true)
        (if (Utilities|Enum|Equal(Enum) (Variables|Default|GetCharaterState) "ECS_Crouching")
          (Animation|Montage|MontagePlay _returnvalue "/Game/BluePrints/Animation/Player/AM_CrouchThrow.AM_CrouchThrow" 1.0 "MontageLength" 0.0 true)
          (else
            (Animation|Montage|MontagePlay _returnvalue "/Game/BluePrints/Animation/Player/AM_ThrowWeapon.AM_ThrowWeapon" 1.0 "MontageLength" 0.0 true)))
        (CallFunction|ShowProjectTilePath)
        (bind _returnvalue_3 (Game|SpawnActorfromClass "/Game/BluePrints/Player/BP_Grenade.BP_Grenade_C" (Math|Transform|MakeTransform (Transformation|GetSocketLocation (Variables|Character|GetMesh) "mixamorig_RightHandIndex2") "0, 0, 0" "1.000000,1.000000,1.000000") "AdjustIfPossibleButDontSpawnIfColliding" "MultiplyWithRoot" 0 0))
        (Transformation|AttachComponentToComponent _returnvalue_3 (Variables|Character|GetMesh) "mixamorig_RightHandIndex2" "SnapToTarget" "SnapToTarget" "KeepWorld" true))))
  (:Released
    (if _returnvalue_2
      (Variables|Default|SetThrowing false)
      (if (Utilities|Enum|Equal(Enum) (Variables|Default|GetCharaterState) "ECS_Crouching")
        (Ability|Animation|MontageJumptoSection _returnvalue "Throw" "/Game/BluePrints/Animation/Player/AM_CrouchThrow.AM_CrouchThrow")
        (else
          (Ability|Animation|MontageJumptoSection _returnvalue "Throw" "/Game/BluePrints/Animation/Player/AM_ThrowWeapon.AM_ThrowWeapon")))
      (Utilities|FlowControl|Delay 0.2)
      (Utilities|IsValid _bp_grenade
        (:Is%20Valid
          (Default|Throw _bp_grenade (Utilities|ThrowVelicity))
          (Variables|Default|SetMolotovcocktailNum (- (Variables|Default|GetMolotovcocktailNum) 1)))))))

(fn ConstructionScript)